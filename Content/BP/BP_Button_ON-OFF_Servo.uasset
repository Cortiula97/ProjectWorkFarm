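; A physical toggle button that switches a smart farm servo on and off over MQTT.
; When a MetaPawn overlaps the box, the cylinder sinks and a boolean flips, alternately publishing ON or OFF to the servo control topic and swapping the cylinder's material to show the state.
; When the pawn leaves the box, the cylinder returns to its start position.
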(event `self.Box.OnComponentBeginOverlap`
  (params (OverlappedComponent :type "PrimitiveComponent Object Reference") (OtherActor :type "Actor Object Reference") (OtherComp :type "PrimitiveComponent Object Reference") (OtherBodyIndex :type Integer) (bFromSweep :type Boolean) (SweepResult :type "HitResult Structure (by ref)"))
  (bind _mqtt_client (`self.Mqtt Client`))
  (cast `/Game/MY_BP/PAWN/MetaPawn` OtherActor)
  (`KismetSystemLibrary.MoveComponentTo` (`self.Button_Cylinder`) (- (`self.Start`) (0.0 0.0 3.0)))
  (if (`self.Condition`)
    (`DTMqttClient.Publish` _mqtt_client "SmartFarm/Controllo/Servo" "ON" "QoS0" false)
    (set `self.Condition` false)
    (`PrimitiveComponent.SetMaterial` (`self.Button_Cylinder`) 0 "/Game/BP/Green.Green")
    (else
      (`DTMqttClient.Publish` _mqtt_client "SmartFarm/Controllo/Servo" "OFF" "QoS0" false)
      (set `self.Condition` true)
      (`PrimitiveComponent.SetMaterial` (`self.Button_Cylinder`) 0 "/Game/BP/Material_001.Material_001"))))

(event `self.Box.OnComponentEndOverlap`
  (params (OverlappedComponent :type "PrimitiveComponent Object Reference") (OtherActor :type "Actor Object Reference") (OtherComp :type "PrimitiveComponent Object Reference") (OtherBodyIndex :type Integer))
  (cast `/Game/MY_BP/PAWN/MetaPawn` OtherActor)
  (`KismetSystemLibrary.MoveComponentTo` (`self.Button_Cylinder`) (`self.Start`)))

(fn `UserConstructionScript`)