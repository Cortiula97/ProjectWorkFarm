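; BP_Color is an actor that shows the SmartFarm pump control state through the color of its ButtonCylinder mesh.
; On BeginPlay it subscribes to the pump's MQTT control topic and binds a message handler.
; The handler switches the cylinder to the Green material on an "ON" message and to Material_001 for any other payload.
; It only listens to MQTT and never publishes.
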(event `self.ReceiveBeginPlay`
  (`DTMqttClient.Subscribe` (`self.Mqtt Client`) "SmartFarm/Controllo/Pompa" "QoS0")
  (`DTMqttClient.BindMessageDelegate` (`self.Mqtt Client`) (delegate `CustomEvent`)))

(event `CustomEvent`
  (params (Topic :type String) (Message :type String))
  (if (`KismetStringLibrary.EqualEqual_StrStr` Message "ON")
    (`PrimitiveComponent.SetMaterial` (`self.Button_Cylinder`) 0 "/Game/BP/Green.Green")
    (else
      (`PrimitiveComponent.SetMaterial` (`self.Button_Cylinder`) 0 "/Game/BP/Material_001.Material_001"))))

(fn `UserConstructionScript`)