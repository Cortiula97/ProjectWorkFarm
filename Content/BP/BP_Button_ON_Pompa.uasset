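; VR-style push button that switches the SmartFarm pump ON over MQTT.
; A MetaPawn overlapping the Box sinks the button cylinder, publishes ON to the pump control topic unless already flagged on, then binds the message delegate; ending overlap raises it.
; Incoming messages on that topic set the flag and material, green for ON, so the button follows broker state once bound.
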(event `self.ReceiveBeginPlay`)

(event `self.Box.OnComponentBeginOverlap`
  (params (OverlappedComponent :type "PrimitiveComponent Object Reference") (OtherActor :type "Actor Object Reference") (OtherComp :type "PrimitiveComponent Object Reference") (OtherBodyIndex :type Integer) (bFromSweep :type Boolean) (SweepResult :type "HitResult Structure (by ref)"))
  (set `self.Start` (`SceneComponent.RelativeLocation` (`self.Button_Cylinder`)))
  (cast `/Game/MY_BP/PAWN/MetaPawn` OtherActor)
  (`KismetSystemLibrary.MoveComponentTo` (`self.Button_Cylinder`) (- (`self.Start`) (0.0 0.0 3.0)))
  (if (not (`self.Boolean`))
    (`DTMqttClient.Publish` (`self.Mqtt Client`) "SmartFarm/Controllo/Pompa" "ON" "QoS0" false)
    (`DTMqttClient.BindMessageDelegate` (`self.Mqtt Client`) (delegate `OnMessage`))))

(event `OnMessage`
  (params (Topic :type String) (Message :type String))
  (if (`KismetStringLibrary.EqualEqual_StrStr` Topic "SmartFarm/Controllo/Pompa")
    (if (`KismetStringLibrary.EqualEqual_StrStr` Message "ON")
      (`PrimitiveComponent.SetMaterial` (`self.Button_Cylinder`) 0 "/Game/BP/Green.Green")
      (set `self.Boolean` true)
      (else
        (`PrimitiveComponent.SetMaterial` (`self.Button_Cylinder`) 0 "/Game/BP/Material_001.Material_001")
        (set `self.Boolean` false)))))

(event `self.Box.OnComponentEndOverlap`
  (params (OverlappedComponent :type "PrimitiveComponent Object Reference") (OtherActor :type "Actor Object Reference") (OtherComp :type "PrimitiveComponent Object Reference") (OtherBodyIndex :type Integer))
  (cast `/Game/MY_BP/PAWN/MetaPawn` OtherActor)
  (`KismetSystemLibrary.MoveComponentTo` (`self.Button_Cylinder`) (`self.Start`)))

(fn `UserConstructionScript`)